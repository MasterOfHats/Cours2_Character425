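; Player pawn for a platforming movement exercise, with camera-relative movement, jumping and an unfinished wallrun.
; A Walking/Jumping/Falling/Wallrun state machine, driven by SimplePawnMovement's landing, floor-left and apex events, toggles gravity, capsule height and mesh tilt.
; Tick turns the capsule toward horizontal velocity, writes player position to a material parameter collection and sphere-traces for walls.
; Wall validation and hit handling are stubs, so wallrun never starts.
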(event Custom|Handle_OnLanding
  (MovementChange|ChangeMovementState "NewEnumerator0"))

(event Custom|Handle_OnFloorLeft
  (if (Utilities|Enum|NotEqual(Enum) (Variables|Default|GetMovementState) "NewEnumerator1")
    (MovementChange|ChangeMovementState "NewEnumerator2")))

(event Custom|Handle_OnApexReached
  (if (Utilities|Enum|Equal(Enum) (Variables|Default|GetMovementState) "NewEnumerator1")
    (MovementChange|ChangeMovementState "NewEnumerator2")))

(event Custom|StartJump
  (bind _simplepawnmovement (Variables|Default|GetSimplePawnMovement))
  (if (Utilities|Enum|Equal(Enum) (Variables|Default|GetMovementState) "NewEnumerator0")
    (MovementChange|ChangeMovementState "NewEnumerator1")
    (Variables|/Script/Engine.MovementComponent|SetVelocity _simplepawnmovement (Math|Vector|MakeVector (.x (Variables|/Script/Engine.MovementComponent|GetVelocity _simplepawnmovement)) (.y (Variables|/Script/Engine.MovementComponent|GetVelocity _simplepawnmovement)) (Variables|Default|GetJumpZVel)))))

(event Custom|WallHit
  (params (Hit :type Hit%20Result%20Structure)))

(event EventBeginPlay
  (EventDispatchers|BindEventtoOnLanding (Variables|Default|GetSimplePawnMovement) (delegate Custom|Handle_OnLanding))
  (EventDispatchers|BindEventtoOnFloorLeft (Variables|Default|GetSimplePawnMovement) (delegate Custom|Handle_OnFloorLeft))
  (EventDispatchers|AssignOnApexReached (Variables|Default|GetSimplePawnMovement) (delegate Custom|Handle_OnApexReached))
  (Variables|Default|SetOriginalGravityAccel (Variables|/Script/Cours2.SimplePawnMovement|GetGravityAccel (Variables|Default|GetSimplePawnMovement))))

(event EventTick
  (params (DeltaSeconds :type Float%20%28single-precision%29))
  (Utilities|FlowControl|Sequence
    (:then_0
      (|RotateCapsuletoMovement)
      (|SetCollectionParamValues))
    (:then_1
      (CallFunction|DEBUGTick))
    (:then_2
      (if (Utilities|Enum|NotEqual(Enum) (Variables|Default|GetMovementState) "NewEnumerator3")
        (bind (_returnvalue _normal _outhit) (Wall|CheckifGrazingWall 5.0))
        (if _returnvalue
          (CallFunction|WallHit _outhit))))))

(event Input|ActionEvents|InputActionInputJump
  (params (Key :type Key%20Structure))
  (:Pressed
    (CallFunction|StartJump)))

(event Input|AxisEvents|InputAxisMoveForward
  (params (AxisValue :type Float%20%28single-precision%29))
  (if (not (Variables|Default|GetbIgnoreMoveInput))
    (switch Utilities|FlowControl|Switch|SwitchonEMovementState (Variables|Default|GetMovementState)
      (:NewEnumerator0
        _)
      (:NewEnumerator1
        _)
      (:NewEnumerator2
        _))
    (Walking|MoveForwardGround (Input|AxisValues|GetMoveForward))))

(event Input|AxisEvents|InputAxisMoveRight
  (params (AxisValue :type Float%20%28single-precision%29))
  (if (not (Variables|Default|GetbIgnoreMoveInput))
    (switch Utilities|FlowControl|Switch|SwitchonEMovementState (Variables|Default|GetMovementState)
      (:NewEnumerator0
        _)
      (:NewEnumerator1
        _)
      (:NewEnumerator2
        _))
    (Walking|MoveRightGround (Input|AxisValues|GetMoveRight))))

(event Input|AxisEvents|InputAxisCameraUp
  (params (AxisValue :type Float%20%28single-precision%29))
  (Pawn|Input|AddControllerPitchInput AxisValue))

(event Input|AxisEvents|InputAxisCameraRight
  (params (AxisValue :type Float%20%28single-precision%29))
  (Pawn|Input|AddControllerYawInput AxisValue))

(fn ConstructionScript)

(fn GetXYVelocity
  (return (* (Transformation|GetVelocity) "1.000000,1.000000, 0")))

(fn ChangeMovementState
  (params (NewMovementState :type EMovementState%20Enum :default "NewEnumerator0"))
  (LocalVariables|SetOldMovementState (Variables|Default|GetMovementState))
  (bind _output_get (Variables|Default|SetMovementState NewMovementState))
  (Utilities|FlowControl|Sequence
    (:then_0
      ;[0.25 0.25 0.25 0] On entering movement state
      (switch Utilities|FlowControl|Switch|SwitchonEMovementState _output_get
        (:NewEnumerator0
          (Variables|/Script/Cours2.SimplePawnMovement|SetbActiveGravity (Variables|Default|GetSimplePawnMovement) false))
        (:NewEnumerator1
          (Variables|/Script/Cours2.SimplePawnMovement|SetbActiveGravity (Variables|Default|GetSimplePawnMovement) true)
          (Components|Capsule|SetCapsuleHalfHeight (Variables|Default|GetCapsule) 3e+01 true))
        (:NewEnumerator2
          (Variables|/Script/Cours2.SimplePawnMovement|SetbActiveGravity (Variables|Default|GetSimplePawnMovement) true))
        (:NewEnumerator3
          (CallFunction|SetWallRunCosmetic "0, 0, 0"))))
    (:then_1
      ;[0.25 0.25 0.25 0] On exiting movement functionality
      (switch Utilities|FlowControl|Switch|SwitchonEMovementState (LocalVariables|GetOldMovementState)
        (:NewEnumerator1
          (Components|Capsule|SetCapsuleHalfHeight (Variables|Default|GetCapsule) 85.0 true))
        (:NewEnumerator3
          (CallFunction|ResetCosmeticLocation))))))

(fn MoveForwardGround
  (params (AxisValue :type Float%20%28single-precision%29))
  (Pawn|Input|AddMovementInput (Class|KismetMathLibrary|VectorNormal2D (Math|Vector|GetForwardVector (Pawn|GetControlRotation :!class /Script/Engine.Pawn)) 0.0001) (* AxisValue (Variables|Default|GetMoveAccel)) false))

(fn MoveRightGround
  (params (AxisValue :type Float%20%28single-precision%29))
  (Pawn|Input|AddMovementInput (Walking|GetGroundForward) (* AxisValue (Variables|Default|GetMoveAccel)) false))

(fn GetGroundForward
  (return (Class|KismetMathLibrary|VectorNormal2D (Math|Vector|GetRightVector (Pawn|GetControlRotation :!class /Script/Engine.Pawn)) 0.0001)))

(fn CheckifGrazingWall
  (params (ExtraRadius :type Float%20%28single-precision%29))
  (bind _returnvalue (Transformation|GetActorLocation))
  (bind _capsule (Variables|Default|GetCapsule))
  (bind _returnvalue_2 (Components|Capsule|GetScaledCapsuleHalfHeight _capsule))
  (bind (_outhit _returnvalue_3) (Collision|SphereTraceForObjects (- _returnvalue (Math|Vector|MakeVector 0.0 0.0 _returnvalue_2)) (+ _returnvalue (Math|Vector|MakeVector 0.0 0.0 _returnvalue_2)) (+ (Components|Capsule|GetScaledCapsuleRadius (Variables|Default|GetCapsule)) ExtraRadius) (Variables|Default|GetWallObjects) false 0 "None"))
  (if _returnvalue_3
    (if (Wall|IsWallStraight (.ImpactNormal (Collision|BreakHitResult _outhit)))
      (return (Wall|IsWallStraight (.ImpactNormal (Collision|BreakHitResult _outhit))) (.ImpactNormal (Collision|BreakHitResult _outhit)) _outhit))))

(fn IsWallStraight
  (params (Normal :type Vector))
  (return false))

(fn DEBUGTick
  (Development|PrintString (Utilities|String|EnumtoString (Variables|Default|GetMovementState)) true true "(R=0.515625,G=0.147588,B=0.012459,A=1.000000)" 0.0))

(fn StopVelZ
  (bind _returnvalue (Transformation|GetVelocity))
  (Variables|/Script/Engine.MovementComponent|SetVelocity (Variables|Default|GetSimplePawnMovement) (Math|Vector|MakeVector (.x _returnvalue) (.y _returnvalue) 0.0)))

(fn SetWallRunCosmetic
  (params (WallNormal :type Vector))
  (bind _capsule (Variables|Default|GetCapsule))
  (bind _returnvalue (Math|Vector|GetRightVector _capsule))
  (bind _returnvalue_2 (Math|Vector|DotProduct WallNormal _returnvalue))
  (bind _returnvalue_3 (Math|Float|Sign(Float) _returnvalue_2))
  (Transformation|SetRelativeRotation (Variables|Default|GetSkeletalMesh) (Math|Rotator|MakeRotator 0.0 (* 3e+01 _returnvalue_3) -9e+01) false false)
  (Transformation|SetRelativeLocation (Variables|Default|GetSkeletalMesh) (Math|Vector|MakeVector 0.0 (* -2e+01 _returnvalue_3) -9e+01) false false))

(fn ResetCosmeticLocation
  (Transformation|SetRelativeRotation (Variables|Default|GetSkeletalMesh) (Math|Rotator|MakeRotator 0.0 0.0 -9e+01) false false)
  (Transformation|SetRelativeLocation (Variables|Default|GetSkeletalMesh) (Math|Vector|MakeVector 0.0 0.0 -9e+01) false false))